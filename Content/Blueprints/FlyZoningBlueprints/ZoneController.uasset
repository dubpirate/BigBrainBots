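; ZoneController is a registry of flight zones that supplies the target height for flybots based on their position.
; Zones are added through RegisterZone, which stores each one and returns its index.
; GetFlyHeight tests the position against each zone's box component bounds and returns the first match's FlyHeight.
; Outside every zone it returns 200 units below the current height, so the bot keeps descending.
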(fn `GetFlyHeight`
  (params (`FlyBot Position` :type "Vector Structure"))
  (returns (`New Fly Zone` :type "Float (double-precision)"))
  ;[1 1 1] If you're in a zone, return the zone height
  (for _array_element (`self.Zones`)
    (bind (_origin _boxextent) (`KismetSystemLibrary.GetComponentBounds` (`/Game/Blueprints/FlyZoningBlueprints/FlyZone.BoxZone` _array_element)))
    (if (`KismetMathLibrary.IsPointInBox` `FlyBot Position` _origin _boxextent)
      (return (`/Game/Blueprints/FlyZoningBlueprints/FlyZone.Fly Height` _array_element))))
  ;[1 1 1] If the flybot isn't in a zone, just fall until you die.
  (return (- (.z `FlyBot Position`) 200.0)))

(fn `RegisterZone`
  (params (Zone :type "/Game/Blueprints/FlyZoningBlueprints/FlyZone Object Reference"))
  (returns (`Zone Index` :type Integer))
  (`KismetArrayLibrary.Array_Set` (`self.Zones`) (`self.Total Zones`) Zone true)
  (bind _output_get (set `self.Total Zones` (+ (`self.Total Zones`) 1)))
  (return (- _output_get 1)))

(fn `UserConstructionScript`)