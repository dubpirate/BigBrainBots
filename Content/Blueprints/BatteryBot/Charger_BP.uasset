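; Charger actor that charges the BatteryBot when its trigger conditions are met.
; The construction script finds and caches the BatteryBot in the level with GetActorOfClass.
; The BlueprintStuff event calls EvaulateTriggers and, if it passes and the bot is not already Charged, calls ChargeBB on it.
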(event `self.BlueprintStuff`
  (bind _returnvalue (`self.EvaulateTriggers`))
  (if (and _returnvalue (not (`/Game/Blueprints/BatteryBot/BatteryBot.Charged` (`self.BatteryBot`))))
    (`/Game/Blueprints/BatteryBot/BatteryBot.ChargeBB` (`self.BatteryBot`))))

(fn `UserConstructionScript`
  (bind _returnvalue (`GameplayStatics.GetActorOfClass` "/Game/Blueprints/BatteryBot/BatteryBot.BatteryBot_C"))
  (set `self.BatteryBot` _returnvalue))