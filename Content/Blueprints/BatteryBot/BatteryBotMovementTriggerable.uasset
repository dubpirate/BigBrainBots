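; BatteryBotMovementTriggerable is a toggleable trigger that drives the level's BatteryBot to move in a set direction.
; The construction script caches the first BatteryBot actor found in the world.
; The BlueprintStuff event flips the On flag, and while it is set, Tick calls the bot's Move with Direction every frame and prints a debug message.
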(event `self.ReceiveTick`
  (params (DeltaSeconds :type "Float (single-precision)"))
  (if (`self.On`)
    (`/Game/Blueprints/BatteryBot/BatteryBot.Move` (`self.BatteryBot`) (`self.Direction`))
    (`KismetSystemLibrary.PrintString` "BBMoveTrigger has triggered.")))

(event `self.BlueprintStuff`
  (set `self.On` (not (`self.On`))))

(fn `UserConstructionScript`
  (bind _returnvalue (`GameplayStatics.GetActorOfClass` "/Game/Blueprints/BatteryBot/BatteryBot.BatteryBot_C"))
  (set `self.BatteryBot` _returnvalue))