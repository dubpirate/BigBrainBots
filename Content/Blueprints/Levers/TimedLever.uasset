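; TimedLever is a lever actor that switches its state off when its countdown runs out.
; Overlapping its LeverPullRange adds the lever to a StandardBot_BP's InteractableSet, and leaving the range removes it.
; Tick decrements CurrTime while it is positive, then calls SetState(false) and clamps the timer to zero.
; The countdown start and the SetState logic are defined outside these graphs.
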(event `self.Lever Pull Range.OnComponentBeginOverlap`
  (params (OverlappedComponent :type "PrimitiveComponent Object Reference") (OtherActor :type "Actor Object Reference") (OtherComp :type "PrimitiveComponent Object Reference") (OtherBodyIndex :type Integer) (bFromSweep :type Boolean) (SweepResult :type "HitResult Structure (by ref)"))
  (bind _asstandard_bot_bp (cast `/Game/Blueprints/StandardBot_BP` OtherActor))
  (`BlueprintSetLibrary.Set_Add` (`/Game/Blueprints/StandardBot_BP.InteractableSet` _asstandard_bot_bp) self))

(event `self.Lever Pull Range.OnComponentEndOverlap`
  (params (OverlappedComponent :type "PrimitiveComponent Object Reference") (OtherActor :type "Actor Object Reference") (OtherComp :type "PrimitiveComponent Object Reference") (OtherBodyIndex :type Integer))
  (bind _asstandard_bot_bp (cast `/Game/Blueprints/StandardBot_BP` OtherActor))
  (`BlueprintSetLibrary.Set_Remove` (`/Game/Blueprints/StandardBot_BP.InteractableSet` _asstandard_bot_bp) self))

(event `self.ReceiveBeginPlay`)

(event `self.ReceiveTick`
  (params (DeltaSeconds :type "Float (single-precision)"))
  (if (> (`self.CurrTime`) 0.0)
    (set `self.CurrTime` (- (`self.CurrTime`) DeltaSeconds))
    (if (<= (`self.CurrTime`) 0.0)
      (`self.SetState` false)
      (set `self.CurrTime` 0.0))))

(fn `UserConstructionScript`)