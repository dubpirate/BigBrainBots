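; Exit zone Blueprint that detects when four bots have gathered inside it to mark the level as completed.
; Overlap begin and end on its collision component raise and lower an InZone counter for BotParent actors, printing the count each time.
; Tick polls the counter and, at exactly four, prints a completion message after a short Delay.
; The level-opening call is disconnected, so no level transition happens.
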(event `self.ReceiveTick`
  (params (DeltaSeconds :type "Float (single-precision)"))
  (if (== (`self.InZone`) 4)
    (`KismetSystemLibrary.Delay` 2.0)
    (`KismetSystemLibrary.PrintText` "Level Completed")))

(event `self.CollisionComponent.OnComponentBeginOverlap`
  (params (OverlappedComponent :type "PrimitiveComponent Object Reference") (OtherActor :type "Actor Object Reference") (OtherComp :type "PrimitiveComponent Object Reference") (OtherBodyIndex :type Integer) (bFromSweep :type Boolean) (SweepResult :type "HitResult Structure (by ref)"))
  (cast `BotParent` OtherActor)
  (bind _output_get (set `self.InZone` (+ (`self.InZone`) 1)))
  (`KismetSystemLibrary.PrintText` (`KismetTextLibrary.Conv_IntToText` _output_get)))

(event `self.CollisionComponent.OnComponentEndOverlap`
  (params (OverlappedComponent :type "PrimitiveComponent Object Reference") (OtherActor :type "Actor Object Reference") (OtherComp :type "PrimitiveComponent Object Reference") (OtherBodyIndex :type Integer))
  (cast `BotParent` OtherActor)
  (bind _output_get (set `self.InZone` (- (`self.InZone`) 1)))
  (`KismetSystemLibrary.PrintText` (`KismetTextLibrary.Conv_IntToText` _output_get)))

(fn `UserConstructionScript`)