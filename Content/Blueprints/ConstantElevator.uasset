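; Trigger-driven elevator that keeps moving a cube back and forth between its starting position and an EndPoint component while active.
; BeginPlay caches both positions, and BlueprintStuff stores the EvaulateTriggers result in Move to play or reverse SliderTimeline.
; The timeline lerps the cube's world location without sweeping.
; On finish it flips MoveUp and, while Move holds, runs again, pausing briefly before reversing.
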(event `self.BlueprintStuff`
  (bind _returnvalue (`self.EvaulateTriggers`))
  (bind _output_get (set `self.Move` _returnvalue))
  (if _output_get
    (bind (_direction _slidertrack) (`Timeline|SliderTimeline` :!label _label)
      (:`Update`
        (`SceneComponent.K2_SetWorldLocation` (`self.Cube`) (`KismetMathLibrary.VLerp` (`self.StartPos`) (`self.EndPos`) _slidertrack) false false))
      (:`Finished`
        (set `self.MoveUp` (not (`self.MoveUp`)))
        (if (`self.Move`)
          (if (`self.MoveUp`)
            (goto _label)
            (else
              (`KismetSystemLibrary.Delay` 0.4)
              (goto _label :!via `Reverse`))))))
    (else
      (goto _label :!via `Reverse`))))

(event `self.ReceiveBeginPlay`
  (set `self.StartPos` (`SceneComponent.K2_GetComponentLocation` (`self.Cube`)))
  (set `self.EndPos` (`SceneComponent.K2_GetComponentLocation` (`self.EndPoint`)))
  (set `self.MoveUp` true))

(fn `UserConstructionScript`)