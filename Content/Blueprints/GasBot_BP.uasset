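; GasBot is a bot with a deployable anti-gas zone that shields bots from gas, itself starting with a zero gas multiplier.
; It initializes health and binds itself to its health bar widget.
; Interact toggles the zone's state and visibility.
; While deployed, overlap events zero entering bots' gas multipliers and set exiting ones to type-specific values, higher for FlyBots and unchanged for GasBots; toggling doesn't update bots already inside.
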(event `self.ReceiveBeginPlay`
  (set `self.Gas_Multiplier` 0.0)
  (bind _output_get (set `self.Max_Health` 250.0))
  (set `self.Health` _output_get)
  (bind _ashealthbar_bp (cast `/Game/Blueprints/UI/Healthbar_BP` (`WidgetComponent.GetUserWidgetObject` (`self.SB_HealthBar`))))
  (set `/Game/Blueprints/UI/Healthbar_BP.Bot` self _ashealthbar_bp)
  (set `self.gasDep` false))

(event `self.ReceiveTick`
  (params (DeltaSeconds :type "Float (single-precision)")))

(event `InputAction|Interact`
  (params (Key :type "Key Structure"))
  (:`Pressed`
    (bind _output_get (set `self.gasDep` (not (`self.gasDep`))))
    (`SceneComponent.SetVisibility` (`self.Anti_Gas`) _output_get false)))

(event `self.Anti_Gas.OnComponentBeginOverlap`
  (params (OverlappedComponent :type "PrimitiveComponent Object Reference") (OtherActor :type "Actor Object Reference") (OtherComp :type "PrimitiveComponent Object Reference") (OtherBodyIndex :type Integer) (bFromSweep :type Boolean) (SweepResult :type "HitResult Structure (by ref)"))
  (bind _asbot_parent (cast `BotParent` OtherActor))
  (if (`self.gasDep`)
    (set `BotParent.Gas_Multiplier` 0.0 _asbot_parent)))

(event `self.Anti_Gas.OnComponentEndOverlap`
  (params (OverlappedComponent :type "PrimitiveComponent Object Reference") (OtherActor :type "Actor Object Reference") (OtherComp :type "PrimitiveComponent Object Reference") (OtherBodyIndex :type Integer))
  (if (`self.gasDep`)
    (bind _asbot_parent (cast `BotParent` OtherActor))
    (bind _asfly_bot_bp (cast `/Game/Blueprints/FlyBot_BP` _asbot_parent)
      (:`then`
        (set `BotParent.Gas_Multiplier` 5.0 _asfly_bot_bp))
      (:`CastFailed`
        (cast `/Game/Blueprints/GasBot_BP` _asbot_parent
          (:`CastFailed`
            (set `BotParent.Gas_Multiplier` 1.0 _asbot_parent)))))))

(fn `UserConstructionScript`)