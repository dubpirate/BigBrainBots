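; Triggerable bridge actor that slides its Cube out and back according to the state of its triggers.
; BlueprintStuff calls EvaulateTriggers, playing SliderTimeline when true and reversing it when false.
; The timeline lerps the Cube's relative location between StartPos, the actor location cached at BeginPlay, and a fixed offset along Y.
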(event `self.BlueprintStuff`
  (bind _returnvalue (`self.EvaulateTriggers`))
  (if _returnvalue
    (bind (_direction _slidertrack) (`Timeline|SliderTimeline` :!label _label)
      (:`Update`
        (`SceneComponent.K2_SetRelativeLocation` (`self.Cube`) (`KismetMathLibrary.VLerp` (`self.StartPos`) (+ (`self.StartPos`) (0.0 201.0 0.0)) _slidertrack) false false)))
    (else
      (goto _label :!via `Reverse`))))

(event `self.ReceiveBeginPlay`
  (set `self.StartPos` (`self.K2_GetActorLocation`)))

(fn `UserConstructionScript`)