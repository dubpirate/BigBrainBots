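; Elevator actor that carries a group of bots by moving its cube platform to an end point.
; Begin overlaps on the collision component add BotParent actors to a list, which has no removal logic.
; While the list holds exactly four entries, Tick waits briefly, then plays a timeline that lerps the cube from its starting location to the EndPoint location captured at BeginPlay.
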(event `self.ReceiveTick`
  (params (DeltaSeconds :type "Float (single-precision)"))
  (if (== (`BlueprintSetLibrary.Set_Length` (`self.BotsOnElevator`)) 4)
    (`KismetSystemLibrary.Delay` 1.0)
    (bind (_direction _slidertrack) (`Timeline|SliderTimeline`)
      (:`Update`
        (`SceneComponent.K2_SetWorldLocation` (`self.Cube`) (`KismetMathLibrary.VLerp` (`self.StartPos`) (`self.EndPos`) _slidertrack) false false)))))

(event `self.CollisionComponent.OnComponentBeginOverlap`
  (params (OverlappedComponent :type "PrimitiveComponent Object Reference") (OtherActor :type "Actor Object Reference") (OtherComp :type "PrimitiveComponent Object Reference") (OtherBodyIndex :type Integer) (bFromSweep :type Boolean) (SweepResult :type "HitResult Structure (by ref)"))
  (bind _asbot_parent (cast `BotParent` OtherActor))
  (`BlueprintSetLibrary.Set_Add` (`self.BotsOnElevator`) _asbot_parent))

(event `self.ReceiveBeginPlay`
  (set `self.StartPos` (`SceneComponent.K2_GetComponentLocation` (`self.Cube`)))
  (set `self.EndPos` (`SceneComponent.K2_GetComponentLocation` (`self.EndPoint`))))

(fn `UserConstructionScript`)