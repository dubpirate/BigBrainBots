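; WaitElevator is an elevator actor that slides its Cube between its starting position and an EndPoint component's position.
; BeginPlay caches both world positions.
; The BlueprintStuff event checks EvaulateTriggers, playing SliderTimeline when true and reversing it when false.
; The timeline's track drives a position lerp without sweep, so the cube travels out and back with the trigger state.
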(event `self.BlueprintStuff`
  (bind _returnvalue (`self.EvaulateTriggers`))
  (if _returnvalue
    (bind (_direction _slidertrack) (`Timeline|SliderTimeline` :!label _label)
      (:`Update`
        (`SceneComponent.K2_SetWorldLocation` (`self.Cube`) (`KismetMathLibrary.VLerp` (`self.StartPos`) (`self.EndPos`) _slidertrack) false false)))
    (else
      (goto _label :!via `Reverse`))))

(event `self.ReceiveBeginPlay`
  (set `self.StartPos` (`SceneComponent.K2_GetComponentLocation` (`self.Cube`)))
  (set `self.EndPos` (`SceneComponent.K2_GetComponentLocation` (`self.EndPoint`))))

(fn `UserConstructionScript`)