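; Door Blueprint that slides its Cube down once its trigger conditions are met.
; BeginPlay caches the Cube's relative start position.
; The BlueprintStuff event calls EvaulateTriggers, defined outside this graph, and on true plays SliderTimeline, which lerps the Cube to a fixed offset below that start.
; The graph has no reverse or closing path.
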(event `self.BlueprintStuff`
  (bind _returnvalue (`self.EvaulateTriggers`))
  (if _returnvalue
    (bind (_direction _slidertrack) (`Timeline|SliderTimeline`)
      (:`Update`
        (`SceneComponent.K2_SetRelativeLocation` (`self.Cube`) (`KismetMathLibrary.VLerp` (`self.StartPos`) (+ (`self.StartPos`) (0.0 0.0 -60.0)) _slidertrack) false false)))))

(event `self.ReceiveBeginPlay`
  (set `self.StartPos` (`SceneComponent.RelativeLocation` (`self.Cube`))))

(fn `UserConstructionScript`)