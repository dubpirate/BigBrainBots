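; ExitDoor is a sliding double door that opens when its trigger check passes.
; BeginPlay caches the closed positions of the Left and Right panels.
; The BlueprintStuff event calls EvaulateTriggers and, on success, plays SliderTimeline, lerping each panel from its start position to the relative location of its LeftOpen or RightOpen marker component.
; The graph has no closing logic.
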(event `self.BlueprintStuff`
  (bind _returnvalue (`self.EvaulateTriggers`))
  (if _returnvalue
    (bind (_direction _slidertrack) (`Timeline|SliderTimeline`)
      (:`Update`
        (`SceneComponent.K2_SetRelativeLocation` (`self.Right`) (`KismetMathLibrary.VLerp` (`self.StartRight`) (`SceneComponent.RelativeLocation` (`self.RightOpen`)) _slidertrack) false false)
        (`SceneComponent.K2_SetRelativeLocation` (`self.Left`) (`KismetMathLibrary.VLerp` (`self.StartLeft`) (`SceneComponent.RelativeLocation` (`self.LeftOpen`)) _slidertrack) false false)))))

(event `self.ReceiveBeginPlay`
  (set `self.StartLeft` (`SceneComponent.RelativeLocation` (`self.Left`)))
  (set `self.StartRight` (`SceneComponent.RelativeLocation` (`self.Right`))))

(fn `UserConstructionScript`)