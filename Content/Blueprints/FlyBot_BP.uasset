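; FlyBot_BP is a flying bot actor with a health pool shown on a Healthbar_BP widget.
; BeginPlay fills health and links the widget to the bot, while ChangeHealth applies an unclamped delta and pushes the result to it.
; Tick offsets the actor from the Cone's position by a sine of DeltaSeconds, so it creeps upward rather than bobbing.
; An unconnected trace-and-force hover setup never runs.
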(event `self.ReceiveBeginPlay`
  (bind _output_get (set `self.Max_Health` 250.0))
  (set `self.Health` _output_get)
  (bind _ashealthbar_bp (cast `/Game/Blueprints/Healthbar_BP` (`WidgetComponent.GetUserWidgetObject` (`self.SB_HealthBar`))))
  (set `/Game/Blueprints/Healthbar_BP.Bot` self _ashealthbar_bp))

(event `self.ReceiveTick`
  (params (DeltaSeconds :type "Float (single-precision)"))
  (`self.K2_SetActorLocation` (+ (`KismetMathLibrary.MakeVector` 0.0 0.0 (* (`KismetMathLibrary.Sin` DeltaSeconds) 50.0)) (`SceneComponent.K2_GetComponentLocation` (`self.Cone`)))))

(fn `ChangeHealth`
  (params (DeltaHealth :type "Float (double-precision)"))
  (bind _output_get (set `self.Health` (+ DeltaHealth (`self.Health`))))
  (bind _ashealthbar_bp (cast `/Game/Blueprints/Healthbar_BP` (`WidgetComponent.GetUserWidgetObject` (`self.SB_HealthBar`))))
  (set `/Game/Blueprints/Healthbar_BP.HB_Health` _output_get _ashealthbar_bp))

(fn `UserConstructionScript`)